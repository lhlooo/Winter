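; SaveGame Blueprint that holds the persistent state of a day-based game with house, lake and plain locations.
; It stores day counters, weather, energy, volume, inventory, per-location items and events, current place, and dog and human elapsed times.
; SetPerams copies all values into its variables in one call, and GetParams returns them all, with no other logic or disk access in these functions.
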(fn SetPerams
  (params (TatolDate :type Integer) (PassedDate :type Integer) (Items :type Array%20of%20Winter%20Item%20Structures) (Energy :type Float%20%28double-precision%29) (Weather :type Weather%20Enum :default "SunnyDay") (ItemsInHouse :type Array%20of%20Winter%20Item%20Structures) (itemsInLake :type Array%20of%20Winter%20Item%20Structures) (itemsInPlain :type Array%20of%20Winter%20Item%20Structures) (MaxEnegy :type Float%20%28double-precision%29) (Volume :type Integer) (MaxVolume :type Integer) (HouseEvent :type Array%20of%20Winter%20Event%20Resource%20Structures) (LakeEvent :type Array%20of%20Winter%20Event%20Resource%20Structures) (PlainEvent :type Array%20of%20Winter%20Event%20Resource%20Structures) (CreateEvent :type Array%20of%20Winter%20Event%20Resource%20Structures) (SnowDay :type Integer) (Place :type Place%20Enum :default "House") (PlaceIdx :type Integer) (DogPassedTime :type Float%20%28double-precision%29) (HumanPassedTime :type Float%20%28double-precision%29))
  (Utilities|FlowControl|Sequence
    (:then_0
      (Variables|Default|SetTotalDate TatolDate))
    (:then_1
      (Variables|Default|SetPassedDate PassedDate))
    (:then_2
      (Variables|Default|SetItems Items))
    (:then_3
      (Variables|Default|SetEnergy Energy))
    (:then_4
      (Variables|Default|SetWeather Weather))
    (:then_5
      (Variables|Default|SetItemsInHouse ItemsInHouse))
    (:then_6
      (Variables|Default|SetItemsInLake itemsInLake))
    (:then_7
      (Variables|Default|SetItemsInPlain itemsInPlain))
    (:then_8
      (Variables|Default|SetMaxEnegy MaxEnegy))
    (:then_9
      (Variables|Default|SetVolume Volume))
    (:then_10
      (Variables|Default|SetMaxVolume MaxVolume))
    (:then_11
      (Variables|Default|SetHouseEvent HouseEvent))
    (:then_12
      (Variables|Default|SetLakeEvent LakeEvent))
    (:then_13
      (Variables|Default|SetPlainEvent PlainEvent))
    (:then_14
      (Variables|Default|SetCreateEvent CreateEvent))
    (:then_15
      (Variables|Default|SetSnowDay SnowDay))
    (:then_16
      (Variables|Default|SetPlace Place))
    (:then_17
      (Variables|Default|SetPlaceIdx PlaceIdx))
    (:then_18
      (Variables|Default|SetDogPassedTime DogPassedTime))
    (:then_19
      (Variables|Default|SetHumanPassedTime HumanPassedTime))))

(fn GetParams
  (return (Variables|Default|GetTotalDate) (Variables|Default|GetPassedDate) (Variables|Default|GetItems) (Variables|Default|GetEnergy) (Variables|Default|GetWeather) (Variables|Default|GetItemsInHouse) (Variables|Default|GetItemsInLake) (Variables|Default|GetItemsInPlain) (Variables|Default|GetMaxEnegy) (Variables|Default|GetVolume) (Variables|Default|GetMaxVolume) (Variables|Default|GetHouseEvent) (Variables|Default|GetLakeEvent) (Variables|Default|GetPlainEvent) (Variables|Default|GetCreateEvent) (Variables|Default|GetSnowDay) (Variables|Default|GetPlace) (Variables|Default|GetPlaceIdx) (Variables|Default|GetDogPassedTime) (Variables|Default|GetHumanPassedTime)))