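; Game state for a winter survival-style game, holding day progress, weather, location items and events, and dog and human pass times.
; GetEvents fills the create, house, lake and plain event arrays from DataTables.
; NextDay resets pass times and rolls new weather, or calls End on the winter player controller once the last day passes.
; Weather uses quota-based odds aiming for ten heavy-snow days in thirty, otherwise randomly picking light snow or sun.
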(event EventBeginPlay)

(event EventTick
  (params (DeltaSeconds :type Float%20%28single-precision%29)))

(fn ConstructionScript)

(fn InitParams
  (params (TotalDate :type Integer) (PassedDate :type Integer) (DayWeather :type Weather%20Enum :default "SunnyDay") (HouseItems :type Array%20of%20Winter%20Item%20Structures) (LakeItems :type Array%20of%20Winter%20Item%20Structures) (PlainItems :type Array%20of%20Winter%20Item%20Structures) (HouseEvent :type Array%20of%20Winter%20Event%20Resource%20Structures) (LakeEvent :type Array%20of%20Winter%20Event%20Resource%20Structures) (PlainEvent :type Array%20of%20Winter%20Event%20Resource%20Structures) (CreateEvent :type Array%20of%20Winter%20Event%20Resource%20Structures) (SnowDay :type Integer) (Dog%20Pass%20Time :type Float%20%28single-precision%29) (Human%20Pass%20Time :type Float%20%28single-precision%29))
  (Variables|Default|SetTotalDate TotalDate)
  (Variables|Default|SetPassedDate PassedDate)
  (Variables|Default|SetDayWeather DayWeather)
  (Variables|Default|SetHouseItems HouseItems)
  (Variables|Default|SetLakeItems LakeItems)
  (Variables|Default|SetPlainItems PlainItems)
  (Variables|Default|SetHouseEvent HouseEvent)
  (Variables|Default|SetLakeEvent LakeEvent)
  (Variables|Default|SetPlainEvent PlainEvent)
  (Variables|Event|SetCreateEvent CreateEvent)
  (Variables|Default|SetSnowDay SnowDay)
  (Variables|Default|SetDogPassTime Dog%20Pass%20Time)
  (Variables|Default|SetHumanPassTime Human%20Pass%20Time))

(fn GetEvents
  (bind _houseevents (Variables|Default|GetHouseEvents))
  (bind _createevents (Variables|Default|GetCreateEvents))
  (bind _lakeevents (Variables|Default|GetLakeEvents))
  (bind _plainevents (Variables|Default|GetPlainEvents))
  (Utilities|FlowControl|Sequence
    (:then_0
      (bind _outrownames (DataTable|GetDataTableRowNames _createevents))
      (for _array_element _outrownames
        (bind _returnvalue (Utilities|GetDataTableRow _createevents _array_element)
          (:then
            (Utilities|Array|Add (Variables|Event|GetCreateEvent) _returnvalue)))))
    (:then_1
      (bind _outrownames_2 (DataTable|GetDataTableRowNames _houseevents))
      (for _array_element_2 _outrownames_2
        (bind _returnvalue_2 (Utilities|GetDataTableRow _houseevents _array_element_2)
          (:then
            (Utilities|Array|Add (Variables|Default|GetHouseEvent) _returnvalue_2)))))
    (:then_2
      (bind _outrownames_3 (DataTable|GetDataTableRowNames _lakeevents))
      (for _array_element_3 _outrownames_3
        (bind _returnvalue_3 (Utilities|GetDataTableRow _lakeevents _array_element_3)
          (:then
            (Utilities|Array|Add (Variables|Default|GetLakeEvent) _returnvalue_3))))
      (Variables|Default|SetLakeEventNum (Utilities|Array|Length (Variables|Default|GetLakeEvent))))
    (:then_3
      (bind _outrownames_4 (DataTable|GetDataTableRowNames _plainevents))
      (for _array_element_4 _outrownames_4
        (bind _returnvalue_4 (Utilities|GetDataTableRow _plainevents _array_element_4)
          (:then
            (Utilities|Array|Add (Variables|Default|GetPlainEvent) _returnvalue_4))))
      (Variables|Default|SetPlainEventNum (Utilities|Array|Length (Variables|Default|GetPlainEvent))))))

(fn NextDay
  (bind _output_get (Variables|Default|SetPassedDate (+ (Variables|Default|GetPassedDate) 1)))
  (if (!= _output_get (+ (Variables|Default|GetTotalDate) 1))
    (Variables|Default|SetDogPassTime 0.0)
    (Variables|Default|SetHumanPassTime 0.0)
    (CallFunction|Weather)
    (else
      (Default|End (.AsBP%20Winter%20Player%20Controller (Utilities|Casting|CastToBP_WinterPlayerController (Game|GetPlayerController 0)))))))

(fn Weather
  (if (>= (/ (Math|Conversions|ToFloat(Integer) (- 10 (Variables|Default|GetSnowDay))) (Math|Conversions|ToFloat(Integer) (- 30 (Variables|Default|GetPassedDate)))) (Math|Random|RandomFloatinRange 0.0 1.0))
    (Variables|Default|SetSnowDay (+ (Variables|Default|GetSnowDay) 1))
    (Variables|Default|SetDayWeather "HeavySnow")
    (elif (>= (Math|Random|RandomFloatinRange 0.0 1.0) 0.5)
      (Variables|Default|SetDayWeather "LightSnow")
      (else
        (Variables|Default|SetDayWeather "SunnyDay")))))