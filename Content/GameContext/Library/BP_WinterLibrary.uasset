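; Blueprint function library that gives the energy and time cost of travel between the House, IceLake and IcePlain locations in the winter game.
; Both functions hard-code the same symmetric cost table as nested branches, with zero cost for staying in place.
; DistanceCalculate takes place values, while DistanceCalculateByIdx duplicates the lookup using integer indices 0 to 2.
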(fn DistanceCalculate
  (params (SourcePlace :type Place%20Enum :default "House") (AimPlace :type Place%20Enum :default "House"))
  (if (Utilities|Enum|Equal(Enum) SourcePlace "House")
    (if (Utilities|Enum|Equal(Enum) AimPlace "House")
      (return 0.0 0.0)
      (elif (Utilities|Enum|Equal(Enum) AimPlace "IceLake")
        (return 3e+01 1.5)
        (elif (Utilities|Enum|Equal(Enum) AimPlace "IcePlain")
          (return 2e+01 1.0))))
    (elif (Utilities|Enum|Equal(Enum) SourcePlace "IceLake")
      (if (Utilities|Enum|Equal(Enum) AimPlace "House")
        (return 3e+01 1.5)
        (elif (Utilities|Enum|Equal(Enum) AimPlace "IceLake")
          (return 0.0 0.0)
          (elif (Utilities|Enum|Equal(Enum) AimPlace "IcePlain")
            (return 15.0 0.5))))
      (elif (Utilities|Enum|Equal(Enum) SourcePlace "IcePlain")
        (if (Utilities|Enum|Equal(Enum) AimPlace "House")
          (return 2e+01 1.0)
          (elif (Utilities|Enum|Equal(Enum) AimPlace "IceLake")
            (return 15.0 0.5)
            (elif (Utilities|Enum|Equal(Enum) AimPlace "IcePlain")
              (return 0.0 0.0))))))))

(fn DistanceCalculatebyIdx
  (params (SourceIdx :type Integer) (AimIdx :type Integer))
  (if (== SourceIdx 0)
    (if (== AimIdx 0)
      (return 0.0 0.0)
      (elif (== AimIdx 1)
        (return 3e+01 1.5)
        (elif (== AimIdx 2)
          (return 2e+01 1.0))))
    (elif (== SourceIdx 1)
      (if (== AimIdx 0)
        (return 3e+01 1.5)
        (elif (== AimIdx 1)
          (return 0.0 0.0)
          (elif (== AimIdx 2)
            (return 15.0 0.5))))
      (elif (== SourceIdx 2)
        (if (== AimIdx 0)
          (return 2e+01 1.0)
          (elif (== AimIdx 1)
            (return 15.0 0.5)
            (elif (== AimIdx 2)
              (return 0.0 0.0))))))))